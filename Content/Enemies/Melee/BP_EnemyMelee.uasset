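; Melee enemy Blueprint that damages a Pavlov player character on contact with its HurtBox.
; An overlap sends weapon hit data to the player through OnShot, using the configured on-hit damage.
; The enemy then launches itself away from the player with a tunable upward bonus and disables the HurtBox.
; SetHurtBoxEnabled toggles the box between query-only and no collision; nothing in this file re-enables it.
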(event `self.HurtBox.OnComponentBeginOverlap`
  (params (OverlappedComponent :type "PrimitiveComponent Object Reference") (OtherActor :type "Actor Object Reference") (OtherComp :type "PrimitiveComponent Object Reference") (OtherBodyIndex :type Integer) (bFromSweep :type Boolean) (SweepResult :type "HitResult Structure (by ref)"))
  (bind _asbp_pavlov_character (cast `/Game/Player/Character/BP_PavlovCharacter` OtherActor))
  (`/Engine/EditorBlueprintResources/StandardMacros.IsValid` _asbp_pavlov_character
    (:`Is Valid`
      (`/Game/Shootables/BPI_Shootable.OnShot` _asbp_pavlov_character self "NewEnumerator1" (make `/Game/Weapons/S_WeaponHitData` (`self.OnHitDamage`) 1.0 1.0 1.0))
      (`/Engine/EditorBlueprintResources/StandardMacros.IsValid` _asbp_pavlov_character
        (:`Is Valid`
          (`self.LaunchCharacter` (* (+ (`KismetMathLibrary.Normal` (- (`self.K2_GetActorLocation`) (`self.K2_GetActorLocation` _asbp_pavlov_character))) (`KismetMathLibrary.MakeVector` 0.0 0.0 (`self.OnHitVelocityZBonus`))) (`self.OnHitVelocityFactor`)) true)
          (`self.SetHurtBoxEnabled` false))))))

(fn `SetHurtBoxEnabled`
  (params (Active :type Boolean))
  (`PrimitiveComponent.SetCollisionEnabled` (`self.HurtBox`) (select `bool` Active :`false` "NoCollision" :`true` "QueryOnly" :!type "ECollisionEnabled Enum")))

(fn `UserConstructionScript`
  (`parent.UserConstructionScript`))