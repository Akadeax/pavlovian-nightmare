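; Networked enemy that finds the closest player, computes aim angles toward a target and fires hitscan shots.
; The server spawns its controller; helper functions set heading and pitch variables, and TryShoot gates fire by a delay timer.
; Shots trace from the muzzle and send a damage message to the hit actor, with effects via client events.
; Hits reduce health, destroying the enemy or flashing its dynamic material through a timeline.
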(event `self.ReceiveBeginPlay`
  (bind _returnvalue (`KismetMaterialLibrary.CreateDynamicMaterialInstance` "/Game/Enemies/Assets/M_Enemy.M_Enemy"))
  (bind _output_get (set `self.EnemyMaterial` _returnvalue))
  (`PrimitiveComponent.SetMaterial` (`self.Mesh`) 0 _output_get)
  (`/Engine/EditorBlueprintResources/ActorMacros.Switch Has Authority`
    (:`Authority`
      (`self.SpawnDefaultController`))))

(event `self.ReceiveTick`
  (params (DeltaSeconds :type "Float (single-precision)"))
  (set `self.TimeSinceLastShot` (+ DeltaSeconds (`self.TimeSinceLastShot`))))

(event `Shoot`
  (params (Direction :type "Vector Structure"))
  (bind _returnvalue (`SceneComponent.GetSocketLocation` (`self.Mesh`) "Muzzle"))
  (`self.Clients_ShootBulletVisual`)
  (bind _outhit (`KismetSystemLibrary.LineTraceSingle` :`Start` _returnvalue :`End` (+ (* Direction 5000.0) _returnvalue) :`TraceChannel` "TraceTypeQuery2" :`DrawDebugType` "ForDuration" :`DrawTime` 1.0))
  (message `/Game/Shootables/BPI_Hittable.OnHit` (`.HitActor` (`GameplayStatics.BreakHitResult` _outhit)) _outhit (`self.Damage`)))

(event `Clients_ShootBulletVisual`
  (`NiagaraFunctionLibrary.SpawnSystemAttached` null (`self.Mesh`) "Muzzle" (0.0 0.0 0.0) (struct :`Yaw` -90.0) "SnapToTargetIncludingScale" false true "AutoRelease"))

(event `/Game/Shootables/BPI_Hittable.OnHit`
  (params (HitResult :type "HitResult Structure") (Damage :type Integer))
  (bind _output_get (set `self.CurrentHealth` (- (`self.CurrentHealth`) Damage)))
  (if (<= _output_get 0)
    (`self.K2_DestroyActor`)
    (else
      (`self.Clients_PlayEnemyFlash`))))

(event `Clients_PlayEnemyFlash`
  (bind (_direction _mix) (`Timeline|Timeline` :!via `PlayFromStart`)
    (:`Update`
      (`MaterialInstanceDynamic.SetVectorParameterValue` (`self.EnemyMaterial`) "BaseColor" (`KismetMathLibrary.LinearColorLerp` (struct :`R` 1.0 :`G` 0.01492 :`A` 1.0) (struct :`R` 1.0 :`G` 0.737096 :`A` 1.0) _mix)))))

(fn `GetAnglesToTarget`
  (params (Target :type "Actor Object Reference"))
  (returns (Heading :type "Float (double-precision)") (Pitch :type "Float (double-precision)"))
  (bind (_returnvalue_x _returnvalue_y _returnvalue_z) (`KismetMathLibrary.BreakVector` (`KismetMathLibrary.Normal` (- (`self.K2_GetActorLocation` Target) (`self.K2_GetActorLocation`)))))
  (`/Engine/EditorBlueprintResources/StandardMacros.IsValid` Target
    (:`Is Valid`
      (return (`KismetMathLibrary.DegAtan2` _returnvalue_y _returnvalue_x) (* (`KismetMathLibrary.DegAsin` _returnvalue_z) -1.0)))
    (:`Is Not Valid`
      (return 0.0 0.0))))

(fn `GetClosestPlayer`
  (returns (ClosestPlayer :type "Pawn Object Reference"))
  (locals (Closest :type "Pawn Object Reference") (ClosestDist :type "Float (double-precision)" :default 9999999999.0))
  (for _index (range (`GameplayStatics.GetNumPlayerStates`))
    (bind _returnvalue (`PlayerState.GetPawn` (`GameplayStatics.GetPlayerState` _index)))
    (bind _returnvalue_2 (`KismetMathLibrary.Vector_DistanceSquared` (`self.K2_GetActorLocation`) (`self.K2_GetActorLocation` _returnvalue)))
    (if (< _returnvalue_2 (`local.ClosestDist`))
      (set `local.ClosestDist` _returnvalue_2)
      (set `local.Closest` _returnvalue)))
  (return (`local.Closest`)))

(fn `RotateToTarget`
  (params (Target :type "Actor Object Reference"))
  (bind (_returnvalue_roll _returnvalue_pitch _returnvalue_yaw) (`KismetMathLibrary.BreakRotator` (`self.K2_GetActorRotation`)))
  (bind (_heading _pitch) (`self.GetAnglesToTarget` Target))
  (set `self.HeadingRotation` (+ _heading (* _returnvalue_yaw -1.0)))
  (set `self.PitchRotation` _pitch))

(fn `TryShoot`
  (params (Direction :type "Vector Structure"))
  (if (>= (`self.TimeSinceLastShot`) (`self.FireDelay`))
    (set `self.TimeSinceLastShot` 0.0)
    (`self.Shoot` (`KismetMathLibrary.Normal` Direction))))

(fn `UserConstructionScript`)