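; BP_EnemySpawner is an enemy spawner that places an instance of EnemyClass around itself each time SpawnEnemy is called.
; Enable sets the Active flag that gates spawning, and Disable clears it.
; Each spawn point is a random direction scaled by SpawnRadius in the spawner's local space, so it lies on a sphere's surface rather than inside.
; Collision handling nudges spawns clear when possible but always spawns.
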(fn `Disable`
  (set `self.Active` false))

(fn `Enable`
  (set `self.Active` true))

(fn `SpawnEnemy`
  (if (`self.Active`)
    (`|SpawnActorFromClass` (`self.EnemyClass`) (`KismetMathLibrary.Conv_VectorToTransform` (`KismetMathLibrary.TransformLocation` (`self.GetTransform`) (* (`KismetMathLibrary.RandomUnitVector`) (`self.SpawnRadius`)))) "AdjustIfPossibleButAlwaysSpawn" "MultiplyWithRoot" null null)))

(fn `UserConstructionScript`)