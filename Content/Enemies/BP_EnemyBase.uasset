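; BP_EnemyBase is a networked enemy Character base that shoots, takes damage and dies at zero health.
; The server spawns its controller and fires line traces with random spread applied in spherical coordinates, sending OnHit messages to hit actors.
; Client events play muzzle, trail and sound effects.
; Non-lethal hits launch it away from the source and flash its dynamic material through a Timeline.
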(event `self.ReceiveBeginPlay`
  (bind _returnvalue (`KismetMaterialLibrary.CreateDynamicMaterialInstance` "/Game/Enemies/Assets/M_Enemy.M_Enemy"))
  (bind _output_get (set `self.EnemyMaterial` _returnvalue))
  (`PrimitiveComponent.SetMaterial` (`self.Mesh`) 0 _output_get)
  (`/Engine/EditorBlueprintResources/ActorMacros.Switch Has Authority`
    (:`Authority`
      (`self.SpawnDefaultController`))))

(event `Clients_ShootEffects`
  (params (Direction :type "Vector Structure"))
  (`NiagaraFunctionLibrary.SpawnSystemAttached` "/Game/Enemies/Assets/FXS_WeaponShoot.FXS_WeaponShoot" (`self.Mesh`) "Muzzle" (0.0 0.0 0.0) (struct :`Yaw` -90.0) "SnapToTarget" false true "AutoRelease")
  (bind _returnvalue (`NiagaraFunctionLibrary.SpawnSystemAtLocation` "/Game/Enemies/Assets/FXS_WeaponBulletTrail.FXS_WeaponBulletTrail" (`SceneComponent.GetSocketLocation` (`self.Mesh`) "Muzzle") (struct) (1.0 1.0 1.0) true true "AutoRelease"))
  (`FXSystemComponent.SetVectorParameter` _returnvalue "Direction" Direction)
  (`GameplayStatics.PlaySoundAtLocation` "/Game/Sounds/SW_WeaponShoot.SW_WeaponShoot" (`self.K2_GetActorLocation`) (struct) 1.0 1.0 0.0 null null null null))

(event `Shoot`
  (params (Direction :type "Vector Structure"))
  (bind _returnvalue (`SceneComponent.GetSocketLocation` (`self.Mesh`) "Muzzle"))
  (`/Engine/EditorBlueprintResources/ActorMacros.Switch Has Authority`
    (:`Authority`
      (bind (_theta _phi) (`self.Cartesian to Spherical` Direction))
      (bind _cartesian (`self.SphericalToCartesian` (+ _theta (* (`KismetMathLibrary.RandomFloatInRange` -1.0 1.0) (`self.ShotInnacuracyRadians`))) (+ _phi (* (`KismetMathLibrary.RandomFloatInRange` -1.0 1.0) (`self.ShotInnacuracyRadians`)))))
      (`self.Clients_ShootEffects` _cartesian)
      (bind _outhit (`KismetSystemLibrary.LineTraceSingle` :`Start` _returnvalue :`End` (+ _returnvalue (* _cartesian 5000.0)) :`TraceChannel` "TraceTypeQuery2" :`DrawDebugType` "ForOneFrame" :`DrawTime` 0.0))
      (message `/Game/Shootables/BPI_Hittable.OnHit` (`.HitActor` (`GameplayStatics.BreakHitResult` _outhit)) self (`self.ShotDamage`)))))

(event `/Game/Shootables/BPI_Hittable.OnHit`
  (params (Source :type "Actor Object Reference") (Damage :type Integer))
  (bind (_returnvalue_x _returnvalue_y) (`KismetMathLibrary.BreakVector` (* (`KismetMathLibrary.Normal` (`KismetMathLibrary.MakeVector` (.x (- (`self.K2_GetActorLocation`) (`self.K2_GetActorLocation` Source))) (.y (- (`self.K2_GetActorLocation`) (`self.K2_GetActorLocation` Source))))) (`self.HitKnockbackHorizontal`))))
  (bind _output_get (set `self.CurrentHealth` (- (`self.CurrentHealth`) Damage)))
  (if (<= _output_get 0)
    (`self.K2_DestroyActor`)
    (else
      (`self.LaunchCharacter` (`KismetMathLibrary.MakeVector` _returnvalue_x _returnvalue_y (`self.HitKnockbackVertical`)) true true)
      (`self.Clients_PlayEnemyFlash`))))

(event `Clients_PlayEnemyFlash`
  (bind (_direction _mix) (`Timeline|Timeline` :!via `PlayFromStart`)
    (:`Update`
      (`MaterialInstanceDynamic.SetVectorParameterValue` (`self.EnemyMaterial`) "BaseColor" (`KismetMathLibrary.LinearColorLerp` (struct :`R` 1.0 :`G` 0.01492 :`A` 1.0) (struct :`R` 1.0 :`G` 0.737096 :`A` 1.0) _mix)))))

(fn `Cartesian to Spherical`
  (params (Cartesian :type "Vector Structure"))
  (returns (Theta :type "Float (double-precision)") (Phi :type "Float (double-precision)"))
  (return (`KismetMathLibrary.Atan2` (.y Cartesian) (.x Cartesian)) (`KismetMathLibrary.Acos` (/ (.z Cartesian) (`KismetMathLibrary.VSize` Cartesian)))))

(fn `SphericalToCartesian`
  (params (Theta :type "Float (double-precision)") (Phi :type "Float (double-precision)"))
  (returns (Cartesian :type "Vector Structure"))
  (bind _returnvalue (`KismetMathLibrary.Sin` Phi))
  (return (`KismetMathLibrary.MakeVector` (* _returnvalue (`KismetMathLibrary.Cos` Theta)) (* _returnvalue (`KismetMathLibrary.Sin` Theta)) (`KismetMathLibrary.Cos` Phi))))

(fn `TryShoot`
  (params (Direction :type "Vector Structure"))
  (set `self.TimeSinceLastShot` 0.0)
  (`self.Shoot` (`KismetMathLibrary.Normal` Direction)))

(fn `UserConstructionScript`)