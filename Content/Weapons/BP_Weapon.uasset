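; Networked hitscan weapon configured by replicated WeaponData, handling firing, magazine ammo, optional limited reserve and reloads.
; The owning player traces from the camera and reports BPI_Shootable hits to the server, which applies normal or headshot damage without re-tracing.
; Fire delay and reload progress advance on Tick, with ammo counted locally.
; Muzzle effects multicast through the server, while hit, crit or miss sounds play locally first, then for other players.
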(event `ShootBullet`
  (bind _playercam (`self.PlayerCam`))
  (bind _weapondata (`self.WeaponData`))
  (bind _returnvalue (`SceneComponent.K2_GetComponentLocation` _playercam))
  (`|ExecutionSequence`
    (:`then_0`
      (`self.Server_ShootBullet`))
    (:`then_1`
      (bind (_outhit _returnvalue_2) (`KismetSystemLibrary.LineTraceSingle` _returnvalue (+ _returnvalue (* (`KismetMathLibrary.GetForwardVector` (`SceneComponent.K2_GetComponentRotation` _playercam)) 5000.0)) "TraceTypeQuery2" false (`|MakeArray` (`self.GetOwner`)) "ForOneFrame" true (struct :`R` 1.0 :`A` 1.0) (struct :`G` 1.0 :`A` 1.0) 0.5))
      (if _returnvalue_2
        (bind (_bblockinghit _binitialoverlap _time _distance _location _impactpoint _normal _impactnormal _physmat _hitactor _hitcomponent _hitbonename) (`GameplayStatics.BreakHitResult` _outhit))
        (bind _asbpi_shootable (cast `/Game/Shootables/BPI_Shootable` _hitactor)
          (:`then`
            (bind _returnvalue_3 (== _hitbonename "Head"))
            (`self.OnShoot` (select `bool` _returnvalue_3 :`false` "NewEnumerator1" :`true` "NewEnumerator2" :!type "/Game/Weapons/E_WeaponHitType Enum"))
            (`self.Server_ShootableHit` _asbpi_shootable _outhit (select `bool` _returnvalue_3 :`false` (`/Game/Weapons/BP_WeaponData.Damage` _weapondata) :`true` (`/Game/Weapons/BP_WeaponData.HeadshotDamage` _weapondata))))
          (:`CastFailed`
            (`self.OnShoot` "NewEnumerator0" :!label _label)))
        (else
          (goto _label))))
    (:`then_2`
      (`/Engine/EditorBlueprintResources/StandardMacros.DecrementInt` (`self.CurrentAmmoLeft`)))))

(event `Server_ShootableHit`
  (params (Shootable :type "/Game/Shootables/BPI_Shootable Interface") (HitResult :type "HitResult Structure") (Damage :type Integer))
  (`/Game/Shootables/BPI_Shootable.OnShot` Shootable HitResult Damage))

(event `Server_ShootBullet`
  (`self.Clients_ShootBulletVisual`))

(event `Clients_ShootBulletVisual`
  (`NiagaraFunctionLibrary.SpawnSystemAttached` "/Game/Weapons/FXS_WeaponShoot.FXS_WeaponShoot" (`self.WeaponMesh`) "Muzzle" (0.0 0.0 0.0) (struct :`Yaw` 180.0) "SnapToTargetIncludingScale"))

(event `self.ReceiveTick`
  (params (DeltaSeconds :type "Float (single-precision)"))
  (bind _returnvalue (+ (`self.ReloadProgress`) (/ DeltaSeconds (`/Game/Weapons/BP_WeaponData.ReloadTime` (`self.WeaponData`)))))
  (`|ExecutionSequence`
    (:`then_0`
      (if (< (`self.TimeSinceLastShot`) (`/Game/Weapons/BP_WeaponData.FireDelay` (`self.WeaponData`)))
        (set `self.TimeSinceLastShot` (+ DeltaSeconds (`self.TimeSinceLastShot`)))))
    (:`then_1`
      (if (< (`self.ReloadProgress`) 1.0)
        (if (>= _returnvalue 1.0)
          (`self.On Reload Done`))
        (set `self.ReloadProgress` _returnvalue)))))

(event `Server_Initialize`
  (params (WeaponData :type "/Game/Weapons/BP_WeaponData Object Reference"))
  (set `self.WeaponData` WeaponData))

(event `RepEvent_WeaponData`
  (`SkeletalMeshComponent.SetSkeletalMeshAsset` (`self.WeaponMesh`) (`/Game/Weapons/BP_WeaponData.Mesh` (`self.WeaponData`))))

(event `self.OnPostNetInit`
  ;[0 0 0] if this weapon is locally owned get local player camera for line traces
  (bind _locally (`self.PlayerLocal` :!label _label_2))
  (if _locally
    (bind _asbp_pavlov_character (cast `/Game/Player/Character/BP_PavlovCharacter` (`self.GetOwner`)))
    (set `self.PlayerCam` (`/Game/Player/Character/BP_PavlovCharacter.PlayerCam` _asbp_pavlov_character))))

(event `self.ReceiveBeginPlay`
  (`|ExecutionSequence`
    (:`then_0`
      ;[0 0 0] if this weapon is locally owned get local player camera for line traces
      (if (`self.HasAuthority`)
        (goto _label_2)))
    (:`then_1`
      (add `self.OnShoot` (delegate `OnShoot_Event`)))))

(event `Unequip`
  (set `self.ReloadProgress` 1.0))

(event `OnShoot_Event` :!signature `self.OnShoot`
  (params (HitType :type "/Game/Weapons/E_WeaponHitType Enum" :default "NewEnumerator0"))
  (`self.PlaySound` (select `/Game/Weapons/E_WeaponHitType` HitType :`NewEnumerator0` "/Game/Sounds/SW_WeaponShoot.SW_WeaponShoot" :`NewEnumerator1` "/Game/Sounds/SW_WeaponHit.SW_WeaponHit" :`NewEnumerator2` "/Game/Sounds/SW_WeaponCrit.SW_WeaponCrit" :!type "SoundBase Object Reference"))
  (`self.Server_PlaySound` "/Game/Sounds/SW_WeaponShoot.SW_WeaponShoot"))

(event `PlaySound`
  (params (Sound :type "SoundBase Object Reference"))
  (bind _audio (`self.Audio`))
  (`AudioComponent.SetSound` _audio Sound)
  (`AudioComponent.Play` _audio 0.0))

(event `Server_PlaySound`
  (params (Sound :type "SoundBase Object Reference"))
  (`self.Clients_PlaySound` Sound))

(event `Clients_PlaySound`
  (params (Sound :type "SoundBase Object Reference"))
  (bind _locally (`self.PlayerLocal`))
  (if (not _locally)
    (`self.PlaySound` Sound)))

(event `RefillAmmo`
  (`self.Owning_RefillAmmo`))

(event `Owning_RefillAmmo`
  (bind _weapondata (`self.WeaponData`))
  (set `self.CurrentAmmoLeft` (`/Game/Weapons/BP_WeaponData.MagazineSize` _weapondata))
  (if (`/Game/Weapons/BP_WeaponData.IsLimitedReserve` _weapondata)
    (set `self.CurrentReserveLeft` (`/Game/Weapons/BP_WeaponData.Reserve` _weapondata))))

(fn `CanBeSwitched`
  (returns (NewParam :type Boolean))
  (return (not (`self.IsShooting`))))

(fn `On Reload Done`
  (locals (AmountToReload :type Integer))
  (if (`/Game/Weapons/BP_WeaponData.IsLimitedReserve` (`self.WeaponData`))
    (set `local.AmountToReload` (`KismetMathLibrary.Min` (`self.CurrentReserveLeft`) (- (`/Game/Weapons/BP_WeaponData.MagazineSize` (`self.WeaponData`)) (`self.CurrentAmmoLeft`))))
    (set `self.CurrentAmmoLeft` (+ (`local.AmountToReload`) (`self.CurrentAmmoLeft`)))
    (set `self.CurrentReserveLeft` (- (`self.CurrentReserveLeft`) (`local.AmountToReload`)))
    (else
      (set `self.CurrentAmmoLeft` (`/Game/Weapons/BP_WeaponData.MagazineSize` (`self.WeaponData`))))))

(fn `OnRep_WeaponData`
  (`self.RepEvent_WeaponData`))

(fn `PlayerLocal`
  (returns (Locally :type Boolean))
  (bind _aspawn (cast `Pawn` (`self.GetOwner`))
    (:`then`
      (return (`Pawn.IsLocallyControlled` _aspawn)))
    (:`CastFailed`
      (return false))))

(fn `TryFire`
  (returns (Success :type Boolean))
  (if (and (not (`self.IsShooting`)) (not (`self.IsReloading`)) (> (`self.CurrentAmmoLeft`) 0))
    (set `self.TimeSinceLastShot` 0.0)
    (`self.ShootBullet`)
    (return true)
    (else
      (return false))))

(fn `TryReload`
  (returns (Success :type Boolean))
  (if (and (not (`self.IsShooting`)) (not (`self.IsReloading`)) (< (`self.CurrentAmmoLeft`) (`/Game/Weapons/BP_WeaponData.MagazineSize` (`self.WeaponData`))))
    (if (`/Game/Weapons/BP_WeaponData.IsLimitedReserve` (`self.WeaponData`))
      (if (> (`self.CurrentReserveLeft`) 0)
        _
        (else
          (return false))))
    (set `self.ReloadProgress` 0.0)
    (return true)
    (else
      (return false))))

(fn `UserConstructionScript`)