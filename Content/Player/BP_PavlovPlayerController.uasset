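; Player controller for the Pavlov player that switches Enhanced Input mapping contexts between gameplay and UI.
; BeginPlay applies the game mappings, which clear all contexts and add the default and weapons contexts at equal priority.
; A separate function clears all contexts and adds only the UI context; nothing in this file calls it.
; Both functions check that the input subsystem is valid and print a debug string.
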(event `self.ReceiveBeginPlay`
  (`self.SetGameMappings`))

(fn `SetGameMappings`
  (bind _returnvalue (subsystem `EnhancedInputLocalPlayerSubsystem`))
  (`/Engine/EditorBlueprintResources/StandardMacros.IsValid` _returnvalue
    (:`Is Valid`
      (`EnhancedInputSubsystemInterface.ClearAllMappings` _returnvalue)
      (`EnhancedInputSubsystemInterface.AddMappingContext` _returnvalue "/Game/Player/Input/IMC_Default.IMC_Default" 0 (struct))
      (`EnhancedInputSubsystemInterface.AddMappingContext` _returnvalue "/Game/Player/Input/IMC_Weapons.IMC_Weapons" 0 (struct))
      (`KismetSystemLibrary.PrintString` "game"))))

(fn `SetUIMappings`
  (bind _returnvalue (subsystem `EnhancedInputLocalPlayerSubsystem`))
  (`/Engine/EditorBlueprintResources/StandardMacros.IsValid` _returnvalue
    (:`Is Valid`
      (`EnhancedInputSubsystemInterface.ClearAllMappings` _returnvalue)
      (`EnhancedInputSubsystemInterface.AddMappingContext` _returnvalue "/Game/Player/Input/IMC_UI.IMC_UI" 0 (struct))
      (`KismetSystemLibrary.PrintString` "ui"))))

(fn `UserConstructionScript`)