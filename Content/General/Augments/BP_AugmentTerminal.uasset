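; BP_AugmentTerminal is an interactable terminal that holds an augment and swaps it with whoever uses it.
; On interact, its AugmentContainer calls SwapAugment with the BPC_AugmentContainer found on the interactor's owner.
; It binds to the container's augment change event at BeginPlay and relays it through its own AugmentChanged dispatcher.
; GetWorldLocation reports the actor's location.
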(event `self.ReceiveBeginPlay`
  (add `/Game/General/Augments/BPC_AugmentContainer.AugmentChanged` (`self.AugmentContainer`) (`|CreateDelegate` :!event `OnAugmentChanged`)))

(event `OnAugmentChanged`
  (params (NewAugment :type "/Game/General/Augments/BP_Augment Object Reference"))
  (`self.AugmentChanged`))

(fn `GetWorldLocation`
  (returns (WorldPos :type "Vector Structure"))
  (return (`self.K2_GetActorLocation`)))

(fn `OnInteract`
  (params (Interactor :type "/Game/Interactables/BP_Interactor Object Reference"))
  (returns (Success :type Boolean))
  (`/Game/General/Augments/BPC_AugmentContainer.SwapAugment` (`self.AugmentContainer`) (`self.GetComponentByClass` (`ActorComponent.GetOwner` Interactor) "/Game/General/Augments/BPC_AugmentContainer.BPC_AugmentContainer_C")))

(fn `UserConstructionScript`)