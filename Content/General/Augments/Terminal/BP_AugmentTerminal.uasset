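; Augment terminal actor that holds an augment in its own AugmentContainer and lets players swap augments with it.
; On interact, it swaps its augment with the BPC_AugmentContainer found on the interactor's owner.
; One second after BeginPlay it seeds the container with DA_AugmentOperator via ClientsSetAugment.
; Container change events are relayed through CallAugmentChanged.
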(event `self.ReceiveBeginPlay`
  (add `/Game/General/Augments/Terminal/BPC_AugmentContainer.AugmentChanged` (`self.AugmentContainer`) (`|CreateDelegate` :!event `OnAugmentChanged`))
  (`KismetSystemLibrary.Delay` 1.0)
  (`/Game/General/Augments/Terminal/BPC_AugmentContainer.Clients_SetAugment` (`self.AugmentContainer`) "/Game/General/Augments/Operator/DA_AugmentOperator.DA_AugmentOperator"))

(event `OnAugmentChanged`
  (params (NewAugment :type "/Game/General/Augments/BP_Augment Object Reference"))
  (`self.AugmentChanged`))

(fn `GetWorldLocation`
  (returns (WorldPos :type "Vector Structure"))
  (return (`self.K2_GetActorLocation`)))

(fn `OnInteract`
  (params (Interactor :type "/Game/Interactables/BP_Interactor Object Reference"))
  (returns (Success :type Boolean))
  (`/Game/General/Augments/Terminal/BPC_AugmentContainer.SwapAugment` (`self.AugmentContainer`) (`self.GetComponentByClass` (`ActorComponent.GetOwner` Interactor) "/Game/General/Augments/Terminal/BPC_AugmentContainer.BPC_AugmentContainer_C")))

(fn `UserConstructionScript`)