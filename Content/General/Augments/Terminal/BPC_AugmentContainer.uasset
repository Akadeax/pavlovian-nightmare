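; Component for the augment terminal that holds one augment and shows its texture on a child billboard.
; BeginPlay caches the first child as that billboard.
; Clients_SetAugment ignores unchanged values, otherwise updates the stored augment and sprite, then fires AugmentChanged.
; SwapAugment exchanges augments between two containers through that same event, and an invalid augment clears the sprite.
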(event `self.ReceiveBeginPlay`
  (bind _asbillboard_component (cast `BillboardComponent` (`self.GetChildComponent` 0))
    (:`then`
      (set `self.Billboard` _asbillboard_component))
    (:`CastFailed`
      (`KismetSystemLibrary.PrintString` "Wtf"))))

(event `Clients_SetAugment`
  (params (NewAugment :type "/Game/General/Augments/BP_Augment Object Reference"))
  (if (not (== NewAugment (`self.CurrentAugment`)))
    (`self.SetAugment` NewAugment)
    (`self.AugmentChanged` NewAugment)))

(fn `SetAugment`
  (params (NewAugment :type "/Game/General/Augments/BP_Augment Object Reference"))
  (bind _billboard (`self.Billboard`))
  (bind _output_get (set `self.CurrentAugment` NewAugment))
  (`/Engine/EditorBlueprintResources/StandardMacros.IsValid` _output_get
    (:`Is Valid`
      (`BillboardComponent.SetSprite` _billboard (`/Game/General/Augments/BP_Augment.Texture` _output_get)))
    (:`Is Not Valid`
      (`BillboardComponent.SetSprite` _billboard null))))

(fn `SwapAugment`
  (params (Other :type "/Game/General/Augments/Terminal/BPC_AugmentContainer Object Reference"))
  (locals (OldAugment :type "/Game/General/Augments/BP_Augment Object Reference"))
  (set `local.OldAugment` (`self.CurrentAugment`))
  (`self.Clients_SetAugment` (`/Game/General/Augments/Terminal/BPC_AugmentContainer.CurrentAugment` Other))
  (`self.Clients_SetAugment` Other (`local.OldAugment`)))