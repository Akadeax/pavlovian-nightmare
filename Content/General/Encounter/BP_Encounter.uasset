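; BP_Encounter is an encounter actor that starts a fight once all players gather in its start zone.
; On BeginPlay it binds to the StartZone's all-players-in-zone event.
; When that fires, it disables the zone on clients, enables every spawner in EnemySpawners, and calls a server resource refill on every BP_PavlovCharacter.
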(event `self.ReceiveBeginPlay`
  (add `/Game/General/Encounter/BP_EncounterStartZone.AllPlayersInZone` (`self.StartZone`) (delegate `Event_AllPlayersInZone`)))

(event `Event_AllPlayersInZone`
  (`|ExecutionSequence`
    (:`then_0`
      (`/Game/General/Encounter/BP_EncounterStartZone.Clients_Disable` (`self.StartZone`)))
    (:`then_1`
      (for _array_element (`self.EnemySpawners`)
        (`/Game/General/Encounter/BP_EnemySpawner.Enable` _array_element)))
    (:`then_2`
      (`self.RefillPlayerResources`))))

(fn `RefillPlayerResources`
  (bind _outactors (`GameplayStatics.GetAllActorsOfClass` "/Game/Player/Character/BP_PavlovCharacter.BP_PavlovCharacter_C"))
  (for _array_element _outactors
    (`/Game/Player/Character/BP_PavlovCharacter.Server_RefillResources` _array_element)))

(fn `UserConstructionScript`)