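; BP_EnemySpawner is an encounter actor that repeatedly spawns BP_Enemy around itself while switched on.
; Enable and Disable set the DoSpawn flag, which Tick checks before entering a five-second Delay that paces the spawns.
; Each spawn lands at a random direction times SpawnRadius in the spawner's local space, and the enemy receives the spawner as its Spawner reference.
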(event `self.ReceiveTick`
  (params (DeltaSeconds :type "Float (single-precision)"))
  (if (`self.DoSpawn`)
    (`KismetSystemLibrary.Delay` 5.0)
    (`|SpawnActorFromClass` "/Game/Enemies/BP_Enemy.BP_Enemy_C" (`KismetMathLibrary.Conv_VectorToTransform` (`KismetMathLibrary.TransformLocation` (`self.GetTransform`) (* (`KismetMathLibrary.RandomUnitVector`) (`self.SpawnRadius`)))) "Undefined" "MultiplyWithRoot" null self null)))

(fn `Disable`
  (set `self.DoSpawn` false))

(fn `Enable`
  (set `self.DoSpawn` true))

(fn `UserConstructionScript`)