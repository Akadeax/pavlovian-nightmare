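; BP_EncounterStartZone is an encounter trigger zone that signals when all players are standing inside it.
; On each begin or end overlap of its Cylinder, it compares the count of overlapping BP_PavlovCharacter actors to the number of player states and fires AllPlayersInZone when they match.
; SetEnabled switches the zone on or off by toggling both the cylinder's query collision and the actor's visibility.
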(event `self.Cylinder.OnComponentEndOverlap`
  (params (OverlappedComponent :type "PrimitiveComponent Object Reference") (OtherActor :type "Actor Object Reference") (OtherComp :type "PrimitiveComponent Object Reference") (OtherBodyIndex :type Integer))
  (if (== (`KismetArrayLibrary.Array_Length` (`PrimitiveComponent.GetOverlappingActors` (`self.Cylinder`) "/Game/Player/Character/BP_PavlovCharacter.BP_PavlovCharacter_C")) (`GameplayStatics.GetNumPlayerStates`)) :!label _label
    (`self.AllPlayersInZone`)))

(event `self.Cylinder.OnComponentBeginOverlap`
  (params (OverlappedComponent :type "PrimitiveComponent Object Reference") (OtherActor :type "Actor Object Reference") (OtherComp :type "PrimitiveComponent Object Reference") (OtherBodyIndex :type Integer) (bFromSweep :type Boolean) (SweepResult :type "HitResult Structure (by ref)"))
  (goto _label))

(event `SetEnabled`
  (params (Enable :type Boolean))
  (`PrimitiveComponent.SetCollisionEnabled` (`self.Cylinder`) (select `bool` Enable :`false` "NoCollision" :`true` "QueryOnly" :!type "ECollisionEnabled Enum"))
  (`self.SetActorHiddenInGame` (not Enable)))

(fn `UserConstructionScript`)