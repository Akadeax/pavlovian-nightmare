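; Test raid first encounter that spawns an enemy and opens an exit door when it completes.
; On encounter start it enables the first enemy spawner, spawns from it, then finishes the encounter after a fixed delay regardless of enemy state.
; The finished event opens the end door.
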(event `self.EncounterStarted`
  (bind _output (`|GetArrayItem` (`self.EnemySpawners`)))
  (`/Game/Enemies/BP_EnemySpawner.Enable` _output)
  (for _ (range 1)
    (`/Game/Enemies/BP_EnemySpawner.SpawnEnemy` _output))
  (`KismetSystemLibrary.Delay` 10.0)
  (`self.FinishEncounter`))

(event `self.EncounterFinished`
  (`/Game/General/EncounterComponents/BP_Door.Open` (`self.EndDoor`)))

(fn `UserConstructionScript`
  (`parent.UserConstructionScript`))