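; BP_TestRaid_First is a timed raid encounter for the test raid that spawns enemy waves and opens an end door when it finishes.
; On start it enables all spawners, spawns a wave, posts a chat message that the Oracles are dormant, then finishes after a fixed delay.
; Each encounter tick waits between waves, then calls SpawnEnemy on randomly picked spawners a configurable number of times.
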(event `self.EncounterStarted`
  (for _array_element (`self.EnemySpawners`)
    (`/Game/Enemies/BP_EnemySpawner.Enable` _array_element))
  (`self.SpawnWave`)
  (`KismetSystemLibrary.Delay` 4.0)
  (`self.SendGameModeChatMessage` "The Oracles are dormant...")
  (`KismetSystemLibrary.Delay` 45.0)
  (`self.FinishEncounter`))

(event `SpawnWave`
  (bind _enemyspawners (`self.EnemySpawners`))
  (for _ (range (+ (`self.SpawnCallsPerWave`) 1))
    (`/Game/Enemies/BP_EnemySpawner.SpawnEnemy` (`|GetArrayItem` _enemyspawners (`KismetMathLibrary.RandomInteger` (`KismetArrayLibrary.Array_Length` _enemyspawners))))))

(event `self.EncounterTick`
  (`KismetSystemLibrary.Delay` (`self.TimeBetweenWaves`))
  (`self.SpawnWave`))

(event `self.EncounterFinished`
  (`/Game/General/EncounterComponents/BP_Door.Open` (`self.EndDoor`)))

(fn `UserConstructionScript`
  (`parent.UserConstructionScript`))