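; Test raid encounter Blueprint that manages a set of doors and augment terminals.
; On BeginPlay it opens every door and binds to each terminal's augment-changed event; EncounterStarted closes the doors.
; A shared change handler pushes the new augment to every terminal's AugmentContainer, keeping them in sync.
; The encounter tick and finish events are empty, so doors are not reopened here.
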(event `self.ReceiveBeginPlay`
  (`parent.ReceiveBeginPlay`)
  (for _array_element (`self.Doors`)
    (`/Game/General/EncounterComponents/BP_Door.Open` _array_element))
  (`self.BindAllTerminals`))

(event `self.EncounterStarted`
  (for _array_element (`self.Doors`)
    (`/Game/General/EncounterComponents/BP_Door.Close` _array_element)))

(event `self.EncounterTick`)

(event `self.EncounterFinished`)

(fn `BindAllTerminals`
  (for _array_element (`self.AugmentTerminals`)
    (add `/Game/General/Augments/BPC_AugmentContainer.AugmentChanged` (`/Game/General/Augments/BP_AugmentTerminal.AugmentContainer` _array_element) (`|CreateDelegate` :!event `OnAnyTerminalChanged`))))

(fn `OnAnyTerminalChanged`
  (params (NewAugment :type "/Game/General/Augments/BP_Augment Object Reference"))
  (for _array_element (`self.AugmentTerminals`)
    (`/Game/General/Augments/BPC_AugmentContainer.Clients_SetAugment` (`/Game/General/Augments/BP_AugmentTerminal.AugmentContainer` _array_element) NewAugment)))

(fn `UserConstructionScript`
  (`parent.UserConstructionScript`))