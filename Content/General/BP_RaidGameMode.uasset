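; Game mode for co-op raids that runs encounters in sequence, checkpoints progress and restarts when every player is dead.
; The first ChoosePlayerStart call initializes the BP_Raid, enables the checkpointed or first encounter, and spawns players there.
; Encounter starts save a per-raid checkpoint to the save game and checkpoint subsystem; finishes enable the next encounter.
; A full wipe reloads the raid level via ServerTravel, freezing time and clearing player input mappings.
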(event `Restart`
  (bind _returnvalue (`|GetDataTableRow` "/Game/General/Raid/DT_RaidData.DT_RaidData" (`/Game/General/Raid/BP_Raid.RaidID` (`self.Raid`)))
    (:`then`
      (`KismetSystemLibrary.ExecuteConsoleCommand` (`KismetStringLibrary.Concat_StrStr` "ServerTravel " (`KismetStringLibrary.Conv_NameToString` (`.LevelPath_15_9C8142C84DB58DDFABB6B188000B6EE3` (break `/Game/General/Raid/S_RaidData` _returnvalue))) "?Listen") null)
      (`GameplayStatics.SetGlobalTimeDilation` 0.0)
      (for _index (range (`GameplayStatics.GetNumPlayerStates`))
        (bind _asbp_pavlov_player_controller (cast `/Game/Player/BP_PavlovPlayerController` (`PlayerState.GetPlayerController` (`GameplayStatics.GetPlayerState` _index))))
        (`/Game/Player/BP_PavlovPlayerController.ClearMappings` _asbp_pavlov_player_controller)))))

(event `self.K2_PostLogin`
  (params (NewPlayer :type "PlayerController Object Reference"))
  (bind _asbp_pavlov_player_controller (cast `/Game/Player/BP_PavlovPlayerController` NewPlayer))
  (add `/Game/Player/BP_PavlovPlayerController.DeadStatusChanged` _asbp_pavlov_player_controller (delegate `Event_DeadStatusChanged`)))

(event `Event_DeadStatusChanged`
  (bind _deadcount (`self.CountDeadPlayers`))
  (if (== _deadcount (`GameplayStatics.GetNumPlayerStates`))
    (`self.Restart`)))

(fn `ChoosePlayerStart`
  (params (Player :type "Controller Object Reference"))
  (returns (ReturnValue :type "Actor Object Reference"))
  (`/Engine/EditorBlueprintResources/StandardMacros.IsValid` (`self.Raid`)
    (:`Is Valid`
      _)
    (:`Is Not Valid`
      (`self.Initialize Raid And Encounters`)))
  (bind _encounter (`self.Get Checkpointed Encounter`))
  (`/Engine/EditorBlueprintResources/StandardMacros.IsValid` _encounter
    (:`Is Valid`
      (return (`/Game/General/Encounter/BP_EncounterStartZone.PlayerStart` (`/Game/General/Encounter/BP_Encounter.StartZone` _encounter))))
    (:`Is Not Valid`
      (return (`/Game/General/Raid/BP_Raid.InitialStart` (`self.Raid`))))))

(fn `CountDeadPlayers`
  (returns (DeadCount :type Integer))
  (locals (CurrentDeadCount :type Integer))
  (for _index (range (`GameplayStatics.GetNumPlayerStates`))
    (bind _asbp_pavlov_player_controller (cast `/Game/Player/BP_PavlovPlayerController` (`PlayerState.GetPlayerController` (`GameplayStatics.GetPlayerState` _index))))
    (if (`/Game/Player/BP_PavlovPlayerController.IsDead` _asbp_pavlov_player_controller)
      (`/Engine/EditorBlueprintResources/StandardMacros.IncrementInt` (`local.CurrentDeadCount`))))
  (return (`local.CurrentDeadCount`)))

(fn `Get Checkpointed Encounter`
  (returns (Encounter :type "/Game/General/Encounter/BP_Encounter Object Reference"))
  (bind _lastcheckpoint (`CheckpointSubsystem.LastCheckpoint` (subsystem `CheckpointSubsystem`)))
  (if (== _lastcheckpoint -1)
    (return null)
    (else
      (return (`|GetArrayItem` (`/Game/General/Raid/BP_Raid.Encounters` (`self.Raid`)) _lastcheckpoint)))))

(fn `GetSaveGame`
  (returns (SaveGame :type "/Game/General/Save/BP_RaidsSaveGame Object Reference"))
  (bind _returnvalue (`GameplayStatics.LoadGameFromSlot` "save"))
  (`/Engine/EditorBlueprintResources/StandardMacros.IsValid` _returnvalue
    (:`Is Valid`
      (bind _asbp_raids_save_game (cast `/Game/General/Save/BP_RaidsSaveGame` _returnvalue))
      (return _asbp_raids_save_game))
    (:`Is Not Valid`
      (bind _returnvalue_2 (`GameplayStatics.CreateSaveGameObject` "/Game/General/Save/BP_RaidsSaveGame.BP_RaidsSaveGame_C"))
      (return _returnvalue_2))))

(fn `Initialize Raid And Encounters`
  (bind _returnvalue (`GameplayStatics.GetActorOfClass` "/Game/General/Raid/BP_Raid.BP_Raid_C"))
  (bind _output_get (set `self.Raid` _returnvalue))
  (`self.SetCheckpointFromSave` (`/Game/General/Raid/BP_Raid.RaidID` _output_get))
  ;[0 0 0] Disable all encounters & bind their events to local functions
  (for _array_element (`/Game/General/Raid/BP_Raid.Encounters` (`self.Raid`))
    (`/Game/General/Encounter/BP_Encounter.SetStatus` _array_element "NewEnumerator0")
    (add `/Game/General/Encounter/BP_Encounter.EncounterFinish` _array_element (`|CreateDelegate` :!event `OnAnyEncounterFinished`))
    (add `/Game/General/Encounter/BP_Encounter.EncounterStart` _array_element (`|CreateDelegate` :!event `OnAnyEncounterStarted`)))
  ;[0 0 0] Enable the first encounter
  (bind _encounter (`self.Get Checkpointed Encounter`))
  (`/Engine/EditorBlueprintResources/StandardMacros.IsValid` _encounter
    (:`Is Valid`
      (`/Game/General/Encounter/BP_Encounter.SetStatus` _encounter "NewEnumerator1"))
    (:`Is Not Valid`
      (`/Game/General/Encounter/BP_Encounter.SetStatus` (`|GetArrayItem` (`/Game/General/Raid/BP_Raid.Encounters` (`self.Raid`))) "NewEnumerator1"))))

(fn `OnAnyEncounterFinished`
  (params (Encounter :type "/Game/General/Encounter/BP_Encounter Object Reference"))
  (bind _encounters (`/Game/General/Raid/BP_Raid.Encounters` (`self.Raid`)))
  (bind _returnvalue (`KismetArrayLibrary.Array_Find` _encounters Encounter))
  (if (== _returnvalue (- (`KismetArrayLibrary.Array_Length` _encounters) 1))
    (`KismetSystemLibrary.PrintString` "Raid finished!" true true (struct :`G` 0.66 :`B` 1.0 :`A` 1.0) 15.0)
    (else
      ;[0 0 0] Enable next encounter
      (`/Game/General/Encounter/BP_Encounter.SetStatus` (`|GetArrayItem` (`/Game/General/Raid/BP_Raid.Encounters` (`self.Raid`)) (+ _returnvalue 1)) "NewEnumerator1"))))

(fn `OnAnyEncounterStarted`
  (params (Encounter :type "/Game/General/Encounter/BP_Encounter Object Reference"))
  (bind _savegame (`self.GetSaveGame`))
  (bind _output_get (set `CheckpointSubsystem.LastCheckpoint` (`KismetArrayLibrary.Array_Find` (`/Game/General/Raid/BP_Raid.Encounters` (`self.Raid`)) Encounter) (subsystem `CheckpointSubsystem`)))
  (`BlueprintMapLibrary.Map_Add` (`/Game/General/Save/BP_RaidsSaveGame.RaidCheckpoints` _savegame) (`/Game/General/Raid/BP_Raid.RaidID` (`self.Raid`)) _output_get)
  (`GameplayStatics.SaveGameToSlot` _savegame "save"))

(fn `SetCheckpointFromSave`
  (params (RaidID :type Name))
  (bind _returnvalue (`GameplayStatics.LoadGameFromSlot` "save"))
  (`/Engine/EditorBlueprintResources/StandardMacros.IsValid` _returnvalue
    (:`Is Valid`
      (bind _asbp_raids_save_game (cast `/Game/General/Save/BP_RaidsSaveGame` _returnvalue)
        (:`then`
          (bind (_value _returnvalue_2) (`BlueprintMapLibrary.Map_Find` (`/Game/General/Save/BP_RaidsSaveGame.RaidCheckpoints` _asbp_raids_save_game) RaidID))
          (if _returnvalue_2
            (set `CheckpointSubsystem.LastCheckpoint` _value (subsystem `CheckpointSubsystem`))
            (else
              ;[0 0 0] Fail, either no checkpoint yet or some error
              (set `CheckpointSubsystem.LastCheckpoint` -1 (subsystem `CheckpointSubsystem`) :!label _label))))
        (:`CastFailed`
          (goto _label))))
    (:`Is Not Valid`
      (goto _label))))

(fn `UserConstructionScript`)