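; BP_ShootPanel is a shootable encounter panel that switches on when hit and reverts after a set active time.
; A shot on an inactive panel triggers activation, followed by a retriggerable delay that leads to deactivation.
; Both state changes route through client events that set the Active flag and swap the cube's material between active and default looks.
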(event `/Game/Shootables/BPI_Shootable.OnShot`
  (params (ShotBy :type "Actor Object Reference") (HitType :type "/Game/Weapons/E_WeaponHitType Enum" :default "NewEnumerator0") (Data :type "/Game/Weapons/S_WeaponHitData Structure"))
  (if (not (`self.Active`))
    (`self.OnActivated` ShotBy)))

(event `OnActivated`
  (params (ActivatedBy :type "Actor Object Reference"))
  (`self.Clients_Activate`)
  (`KismetSystemLibrary.RetriggerableDelay` (`self.ActiveTime`))
  (`self.OnDeactivated`))

(event `OnDeactivated`
  (`self.Clients_Deactivate`))

(event `Clients_Activate`
  (`self.Activate`))

(event `Clients_Deactivate`
  (`self.Deactivate`))

(fn `Activate`
  (set `self.Active` true)
  (`PrimitiveComponent.SetMaterial` (`self.Cube`) 0 (`self.ActiveMaterial`)))

(fn `Deactivate`
  (set `self.Active` false)
  (`PrimitiveComponent.SetMaterial` (`self.Cube`) 0 (`self.PanelMaterial`)))

(fn `UserConstructionScript`)