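; BP_DoorPanel is an encounter panel that controls two lists of doors when activated or deactivated.
; On activation it runs the parent logic, then opens every door in DoorsToOpen and closes every door in DoorsToClose.
; On deactivation it closes the DoorsToOpen doors again but leaves the DoorsToClose doors as they are.
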(event `self.OnActivated`
  (params (ActivatedBy :type "Actor Object Reference"))
  (`parent.OnActivated` ActivatedBy)
  (`|ExecutionSequence`
    (:`then_0`
      (for _array_element (`self.DoorsToOpen`)
        (`/Game/General/EncounterComponents/BP_Door.Open` _array_element)))
    (:`then_1`
      (for _array_element_2 (`self.DoorsToClose`)
        (`/Game/General/EncounterComponents/BP_Door.Close` _array_element_2)))))

(event `self.OnDeactivated`
  (`parent.OnDeactivated`)
  (for _array_element (`self.DoorsToOpen`)
    (`/Game/General/EncounterComponents/BP_Door.Close` _array_element)))

(fn `UserConstructionScript`
  (`parent.UserConstructionScript`))