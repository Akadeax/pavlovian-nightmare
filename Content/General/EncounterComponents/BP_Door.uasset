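; BP_Door is an encounter door that opens and closes by animating the vertical scale of its mesh.
; Open and Close only set the IsOpen flag, whose RepNotify calls DoOpen or DoClose so the animation follows the replicated state.
; A single Timeline drives DoorMesh's Z scale, playing forward to open and reversing to close.
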(event `Open`
  (set `self.IsOpen` true))

(event `DoOpen`
  (bind (_direction _scale) (`Timeline|Timeline` :!label _label)
    (:`Update`
      (`SceneComponent.SetRelativeScale3D` (`self.DoorMesh`) (`KismetMathLibrary.MakeVector` 1.0 1.0 _scale)))))

(event `Close`
  (set `self.IsOpen` false))

(event `DoClose`
  (goto _label :!via `Reverse`))

(fn `OnRep_isOpen`
  (if (`self.IsOpen`)
    (`self.DoOpen`)
    (else
      (`self.DoClose`))))

(fn `UserConstructionScript`)