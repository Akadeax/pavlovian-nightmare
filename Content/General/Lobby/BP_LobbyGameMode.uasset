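; BP_LobbyGameMode is the lobby game mode, which sets up joining players and tracks whether the game can start.
; On BeginPlay it caches the raids save game from the "save" slot.
; PostLogin spawns and possesses a lobby character, flags the locally controlled player as host, and binds to their ready changes.
; Each ready change recounts ready players and broadcasts whether everyone is ready through GameStartableChanged.
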(event `self.ReceiveBeginPlay`
  (bind _returnvalue (`GameplayStatics.LoadGameFromSlot` "save"))
  (bind _asbp_raids_save_game (cast `/Game/General/Save/BP_RaidsSaveGame` _returnvalue))
  (set `self.RaidsSaveGame` _asbp_raids_save_game)
  (`self.GetLobbyGameState`))

(event `self.K2_PostLogin`
  (params (NewPlayer :type "PlayerController Object Reference"))
  (`KismetSystemLibrary.PrintString` (`KismetStringLibrary.Concat_StrStr` (`PlayerState.GetPlayerName` (`Controller.PlayerState` NewPlayer)) " connected.") true true (struct :`G` 0.66 :`B` 1.0 :`A` 1.0) 10.0)
  (bind _returnvalue (`|SpawnActorFromClass` "/Game/General/Lobby/BP_LobbyCharacter.BP_LobbyCharacter_C" (`self.GetTransform`) "Undefined" "MultiplyWithRoot" NewPlayer null))
  (`Controller.Possess` NewPlayer _returnvalue)
  (bind _asbp_lobby_player_state (cast `/Game/General/Lobby/BP_LobbyPlayerState` (`Controller.PlayerState` NewPlayer)))
  (set `/Game/General/Lobby/BP_LobbyPlayerState.IsHost` (`Pawn.IsLocallyControlled` _returnvalue) _asbp_lobby_player_state)
  (add `/Game/General/Lobby/BP_LobbyPlayerState.OnReadyChanged` _asbp_lobby_player_state (delegate `OnReadyChanged`)))

(event `OnReadyChanged`
  (params (NewReady :type Boolean))
  (bind _readycount (`self.CountReadyPlayers`))
  (`self.GameStartableChanged` (== _readycount (`KismetArrayLibrary.Array_Length` (`GameStateBase.PlayerArray` (`GameplayStatics.GetGameState`))))))

(fn `CountReadyPlayers`
  (returns (ReadyCount :type Integer))
  (locals (CurrentCount :type Integer))
  (for _array_element (`GameStateBase.PlayerArray` (`GameplayStatics.GetGameState`))
    (bind _asbp_lobby_player_state (cast `/Game/General/Lobby/BP_LobbyPlayerState` _array_element))
    (if (`/Game/General/Lobby/BP_LobbyPlayerState.Ready` _asbp_lobby_player_state)
      (`/Engine/EditorBlueprintResources/StandardMacros.IncrementInt` (`local.CurrentCount`))))
  (return (`local.CurrentCount`)))

(fn `GetLobbyGameState`
  (returns (GameState :type "/Game/General/Lobby/BP_LobbyGameState Object Reference"))
  (bind _asbp_lobby_game_state (cast `/Game/General/Lobby/BP_LobbyGameState` (`GameplayStatics.GetGameState`)))
  (return _asbp_lobby_game_state))

(fn `UserConstructionScript`)