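; Game mode for encounters that restarts the current level once every player is dead.
; PostLogin binds each BP_PavlovPlayerController's dead-status change to a handler that compares the dead count with the player state count.
; Restart issues a ServerTravel console command for the current level as a listen server, sets global time dilation to zero and clears each controller's mappings.
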(event `Restart`
  (bind _returnvalue (`GameplayStatics.GetCurrentLevelName` true))
  (`KismetSystemLibrary.ExecuteConsoleCommand` (`KismetStringLibrary.Concat_StrStr` "ServerTravel " _returnvalue "?Listen") null)
  (`GameplayStatics.SetGlobalTimeDilation` 0.0)
  (for _index (range (`GameplayStatics.GetNumPlayerStates`))
    (bind _asbp_pavlov_player_controller (cast `/Game/Player/BP_PavlovPlayerController` (`PlayerState.GetPlayerController` (`GameplayStatics.GetPlayerState` _index))))
    (`/Game/Player/BP_PavlovPlayerController.ClearMappings` _asbp_pavlov_player_controller)))

(event `self.K2_PostLogin`
  (params (NewPlayer :type "PlayerController Object Reference"))
  (bind _asbp_pavlov_player_controller (cast `/Game/Player/BP_PavlovPlayerController` NewPlayer))
  (add `/Game/Player/BP_PavlovPlayerController.DeadStatusChanged` _asbp_pavlov_player_controller (delegate `Event_DeadStatusChanged`)))

(event `Event_DeadStatusChanged`
  (bind _deadcount (`self.CountDeadPlayers`))
  (if (== _deadcount (`GameplayStatics.GetNumPlayerStates`))
    (`self.Restart`)))

(fn `CountDeadPlayers`
  (returns (DeadCount :type Integer))
  (locals (CurrentDeadCount :type Integer))
  (for _index (range (`GameplayStatics.GetNumPlayerStates`))
    (bind _asbp_pavlov_player_controller (cast `/Game/Player/BP_PavlovPlayerController` (`PlayerState.GetPlayerController` (`GameplayStatics.GetPlayerState` _index))))
    (if (`/Game/Player/BP_PavlovPlayerController.IsDead` _asbp_pavlov_player_controller)
      (`/Engine/EditorBlueprintResources/StandardMacros.IncrementInt` (`local.CurrentDeadCount`))))
  (return (`local.CurrentDeadCount`)))

(fn `UserConstructionScript`)