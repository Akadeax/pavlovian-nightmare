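; Scene component on a Pawn that tracks nearby actors implementing BPI_Interactable.
; On locally controlled pawns, it binds overlap events on its first child box component to maintain the Overlapped list.
; It exposes HasInteractables and GetClosestInteractable for querying that list.
; The closest search compares squared distances against ClosestDistance but never updates it, so it picks the last element under that threshold.
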(event `self.ReceiveBeginPlay`
  (bind _aspawn (cast `Pawn` (`self.GetOwner` self)))
  (if (`Pawn.IsLocallyControlled` _aspawn)
    (bind _asbox_collision (cast `BoxComponent` (`self.GetChildComponent` 0)))
    (add `PrimitiveComponent.OnComponentBeginOverlap` _asbox_collision (delegate `OnComponentBeginOverlap`))
    (add `PrimitiveComponent.OnComponentEndOverlap` _asbox_collision (delegate `OnComponentEndOverlap`))))

(event `OnComponentEndOverlap`
  (params (OverlappedComponent :type "PrimitiveComponent Object Reference") (OtherActor :type "Actor Object Reference") (OtherComp :type "PrimitiveComponent Object Reference") (OtherBodyIndex :type Integer))
  (bind _asbpi_interactable (cast `/Game/Interactables/BPI_Interactable` OtherActor))
  (`KismetArrayLibrary.Array_RemoveItem` (`self.Overlapped`) _asbpi_interactable))

(event `OnComponentBeginOverlap`
  (params (OverlappedComponent :type "PrimitiveComponent Object Reference") (OtherActor :type "Actor Object Reference") (OtherComp :type "PrimitiveComponent Object Reference") (OtherBodyIndex :type Integer) (bFromSweep :type Boolean) (SweepResult :type "HitResult Structure (by ref)"))
  (bind _asbpi_interactable (cast `/Game/Interactables/BPI_Interactable` OtherActor))
  (`KismetArrayLibrary.Array_Add` (`self.Overlapped`) _asbpi_interactable))

(fn `GetClosestInteractable`
  (returns (Interactable :type "/Game/Interactables/BPI_Interactable Interface"))
  (locals (ClosestDistance :type "Float (double-precision)" :default 99999999999.0) (ClosestInteractable :type "/Game/Interactables/BPI_Interactable Interface"))
  (for _array_element (`self.Overlapped`)
    (bind _worldpos (`/Game/Interactables/BPI_Interactable.GetWorldLocation` _array_element))
    (if (< (`KismetMathLibrary.Vector_DistanceSquared` (`self.K2_GetComponentLocation`) _worldpos) (`local.ClosestDistance`))
      (set `local.ClosestInteractable` _array_element)))
  (return (`local.ClosestInteractable`)))

(fn `HasInteractables`
  (returns (HasInteractables :type Boolean))
  (return (not (`KismetArrayLibrary.Array_IsEmpty` (`self.Overlapped`)))))